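; BP_PickupCube is a cube actor that BP_MotionController picks up and drops.
; Pickup plays an attached sound, turns off mesh physics and attaches the root to the given component, keeping world transform.
; It also starts a three-second timer that force-detaches the cube as a stuck-in-hand fallback, sharing Drop's logic.
; Release leaves physics disabled, and an in-hand guard and destroy call sit unconnected.
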(event `/Game/Blueprints/Character/PickupActorInterface.Pickup`
  (params (AttachTo :type "SceneComponent Object Reference"))
  (bind _staticmesh (`self.StaticMesh`))
  (`KismetSystemLibrary.K2_SetTimerDelegate` (delegate `HandleIsStuck`) 3.0)
  (`GameplayStatics.SpawnSoundAttached` "/Game/NasaEROSVR/Sounds/plastic_pickup_Cue.plastic_pickup_Cue" _staticmesh "None" (0.0 0.0 0.0) (struct) "KeepRelativeOffset" false 1.0 1.0 0.0 null null)
  (`PrimitiveComponent.SetSimulatePhysics` _staticmesh false)
  (`SceneComponent.K2_AttachToComponent` (`self.K2_GetRootComponent`) AttachTo "None" "KeepWorld" "KeepWorld" "KeepWorld" false))

(event `HandleIsStuck`
  (`PrimitiveComponent.SetSimulatePhysics` (`self.StaticMesh`) false :!label _label)
  (`self.K2_DetachFromActor` "KeepWorld" "KeepWorld" "KeepWorld"))

(event `/Game/Blueprints/Character/PickupActorInterface.Drop`
  (goto _label))

(fn `UserConstructionScript`)