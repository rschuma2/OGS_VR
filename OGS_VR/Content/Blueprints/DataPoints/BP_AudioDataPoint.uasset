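; BP_AudioDataPoint is a child data point Blueprint that drives an audio datapoint widget through hand controls and a pedestal button.
; It caches its W_AudioDataPoint widget on begin play and registers itself in the Game Instance as the current audio datapoint on overlap.
; The pedestal press activates the widget and toggles hand controls.
; The right button alternates play and pause, while the left reverses the flip values, deactivates the widget and marks it inactive after a delay.
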(event `self.ChildBeginPlay`
  ;[1 1 1] BeginPlay
  (bind _asw_audio_data_point (cast `/Game/NasaEROSVR/UI/W_AudioDataPoint` (`WidgetComponent.GetUserWidgetObject` (`self.Widget`))))
  (set `self.ThisWidget` _asw_audio_data_point))

(event `self.BoxOverlapFunction`
  ;[1 1 1] BoxOverlapFunction. Extends parent overlap event to set the current specific BP in the Game instance
  (set `/Game/Blueprints/EROS_GameInstance.CurrentAudioDatapoint` self (`self.GIRef`)))

(event `self.StartRButtonAction`
  (bind _thiswidget (`self.ThisWidget`))
  ;[1 1 1] Hand Control Actions
  (`GameplayStatics.PlaySound2D` "/Game/NasaEROSVR/Sounds/MinimalUI/370846__cabled-mess__funny-click-minimal-ui-sounds.370846__cabled-mess__funny-click-minimal-ui-sounds" 1.0 1.0 0.0 null null)
  (`/Engine/EditorBlueprintResources/StandardMacros.FlipFlop`
    (:`A`
      (`/Game/NasaEROSVR/UI/W_AudioDataPoint.PlayDatapoint` _thiswidget))
    (:`B`
      (`/Game/NasaEROSVR/UI/W_AudioDataPoint.PauseDatapoint` _thiswidget))))

(event `self.StartLButtonAction`
  ;[1 1 1] Hand Control Actions
  (`GameplayStatics.PlaySound2D` "/Game/NasaEROSVR/Sounds/MinimalUI/370846__cabled-mess__funny-click-minimal-ui-sounds.370846__cabled-mess__funny-click-minimal-ui-sounds" 1.0 1.0 0.0 null null)
  (set `self.ZFlip` -3.2)
  (set `self.XYFlip` 5.0)
  (`self.ToggleHandControls`)
  (`self.ToggleTextVisibility` false)
  (`/Game/NasaEROSVR/UI/W_AudioDataPoint.DeactivateDatapoint` (`self.ThisWidget`))
  (`KismetSystemLibrary.Delay` 2.0)
  (set `self.bIsInactive` true))

(event `self.StartPedestalButtonPress`
  (set `self.ZFlip` 3.2)
  (set `self.XYFlip` -5.0)
  (`self.ToggleHandControls`)
  (`/Game/NasaEROSVR/UI/W_AudioDataPoint.ActivateDatapoint` (`self.ThisWidget`)))

(fn `UserConstructionScript`
  (`parent.UserConstructionScript`))