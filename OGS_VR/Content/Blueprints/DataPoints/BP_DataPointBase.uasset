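; Base VR data point actor: a pulsing scannable cover that hides a gallery pillar with hand-touch buttons.
; Controller overlaps register it on MotionControllerPawn2; a completed timed scan destroys the cover, then raises and rotates the pillar.
; Box overlap, gated by the game instance's DataPointsUnlocked, passes widget content and audio to game instance and pawn.
; Children fill empty hooks for BeginPlay, overlap and button presses; the gallery save logic is disconnected.
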(event `self.ReceiveBeginPlay`
  ;[1 1 1] BeginPlay - Create game instance ref.
  (bind _aseros_game_instance (cast `/Game/Blueprints/EROS_GameInstance` (`GameplayStatics.GetGameInstance`)))
  (set `self.GIRef` _aseros_game_instance)
  (bind _asmotion_controller_pawn_2 (cast `/Game/Blueprints/MotionControllerPawn2` (`GameplayStatics.GetPlayerCharacter` 0)))
  (set `self.CharRef` _asmotion_controller_pawn_2)
  (bind _returnvalue (`KismetSystemLibrary.K2_SetTimerDelegate` (delegate `HandleScannerPulseTimer`) 0.5 true))
  (set `self.RockPulseTimerHandle` _returnvalue)
  (`self.ChildBeginPlay`))

(event `ScannerPulseTimer`
  ;[1 1 1] ScannerPulseTimer
  (`/Engine/EditorBlueprintResources/StandardMacros.FlipFlop`
    (:`A`
      (`PrimitiveComponent.SetMaterial` (`self.ScannerCoverObject`) 0 "/Game/Megascans/3D_Assets/California_Coastal_Rock_Assembly_00/California_Coastal_Rock_Assembly_00_inst.California_Coastal_Rock_Assembly_00_inst"))
    (:`B`
      (`PrimitiveComponent.SetMaterial` (`self.ScannerCoverObject`) 0 "/Engine/ArtTools/RenderToTexture/Materials/Debug/M_Emissive_Color_0-0-127.M_Emissive_Color_0-0-127"))))

(event `UpdateSaveInformation`
  ;[0 0.9267 1] UpdateSaveInfo (clean up and remove print strings after testing)
)

(event `HandleScannerPulseTimer`
  ;[1 1 1] BeginPlay - Create game instance ref.
  (`self.ScannerPulseTimer`))

(event `SetupWidget`
  ;[1 1 1] SetupBlueprint - Update instance-editable variables locally and on game instance.
  (set `/Game/Blueprints/EROS_GameInstance.CurrentDataPointWidgetClass` (`self.WidgetToLoad`) (`self.GIRef`))
  (`BillboardComponent.SetSprite` (`self.Billboard`) (`self.SpriteToDisplay`))
  (set `/Game/Blueprints/EROS_GameInstance.DataPointImages` (`self.ImagesToDisplay`) (`self.GIRef`))
  (set `/Game/Blueprints/EROS_GameInstance.DataPointTexts` (`self.TextsToDisplay`) (`self.GIRef`)))

(event `self.Box.OnComponentBeginOverlap`
  (params (OverlappedComponent :type "PrimitiveComponent Object Reference") (OtherActor :type "Actor Object Reference") (OtherComp :type "PrimitiveComponent Object Reference") (OtherBodyIndex :type Integer) (bFromSweep :type Boolean) (SweepResult :type "HitResult Structure (by ref)"))
  ;[1 1 1] Begin Overlap - set sound to play on player pawn (audio component) and activate components.
  (set `/Game/Blueprints/EROS_GameInstance.DataPointAudioImg` (`self.SpriteToDisplay`) (`self.GIRef`))
  (bind _asmotion_controller_pawn_2 (cast `/Game/Blueprints/MotionControllerPawn2` OtherActor))
  (if (`/Game/Blueprints/EROS_GameInstance.bDataPointsUnlocked` (`self.GIRef`))
    (`self.SetupWidget`)
    (`AudioComponent.SetSound` (`/Game/Blueprints/MotionControllerPawn2.AudioDataPointComponent` _asmotion_controller_pawn_2) (`self.SoundToPlay`))
    (`ActorComponent.Activate` (`self.activated`) true)
    (`ActorComponent.Deactivate` (`self.deactivated`))
    (`self.BoxOverlapFunction`)
    (else
      (`/Game/Blueprints/MotionControllerPawn2.ShowNotification` (`self.CharRef`) "Additional Ability Required: Gallery Object Scanner" (struct :`R` 1.0 :`B` 0.781225 :`A` 1.0)))))

(event `self.Box.OnComponentEndOverlap`
  (params (OverlappedComponent :type "PrimitiveComponent Object Reference") (OtherActor :type "Actor Object Reference") (OtherComp :type "PrimitiveComponent Object Reference") (OtherBodyIndex :type Integer))
  ;[1 1 1] End Overlap - deactivate components.
  (cast `/Game/Blueprints/MotionControllerPawn2` OtherActor)
  (`ActorComponent.Deactivate` (`self.InterpToMovement`))
  (`ActorComponent.Deactivate` (`self.deactivated`))
  (`ActorComponent.Activate` (`self.deactivated`) true)
  (`ActorComponent.Deactivate` (`self.activated`)))

(event `self.ScannerCoverObject.OnComponentBeginOverlap`
  (params (OverlappedComponent :type "PrimitiveComponent Object Reference") (OtherActor :type "Actor Object Reference") (OtherComp :type "PrimitiveComponent Object Reference") (OtherBodyIndex :type Integer) (bFromSweep :type Boolean) (SweepResult :type "HitResult Structure (by ref)"))
  ;[1 1 1] Begin/End overlap of motion controllers to determine whether a particular datapoint is being pointed at.
  (bind _outactors (`GameplayStatics.GetAllActorsOfClass` "/Game/Blueprints/MotionControllerPawn2.MotionControllerPawn2_C"))
  (bind _output (`|GetArrayItem` _outactors))
  (if (== (`/Game/Blueprints/MotionControllerPawn2.RController` _output) OtherActor)
    (set `/Game/Blueprints/MotionControllerPawn2.bIsPointingAtScanObject` true _output :!label _label)
    (`/Engine/EditorBlueprintResources/StandardMacros.IncrementInt` (`self.NumControllersPointed`)
      (:`  `
        (set `/Game/Blueprints/MotionControllerPawn2.DatapointPointedAt` self _output)))
    (elif (== (`/Game/Blueprints/MotionControllerPawn2.LController` _output) OtherActor)
      (goto _label))))

(event `self.ScannerCoverObject.OnComponentEndOverlap`
  (params (OverlappedComponent :type "PrimitiveComponent Object Reference") (OtherActor :type "Actor Object Reference") (OtherComp :type "PrimitiveComponent Object Reference") (OtherBodyIndex :type Integer))
  ;[1 1 1] Begin/End overlap of motion controllers to determine whether a particular datapoint is being pointed at.
  (bind _outactors (`GameplayStatics.GetAllActorsOfClass` "/Game/Blueprints/MotionControllerPawn2.MotionControllerPawn2_C"))
  (bind _output (`|GetArrayItem` _outactors))
  (if (or (== (`/Game/Blueprints/MotionControllerPawn2.RController` _output) OtherActor) (== (`/Game/Blueprints/MotionControllerPawn2.LController` _output) OtherActor))
    (bind _result (`/Engine/EditorBlueprintResources/StandardMacros.DecrementInt` (`self.NumControllersPointed`))
      (:`  `
        (if (< _result 1)
          (set `/Game/Blueprints/MotionControllerPawn2.bIsPointingAtScanObject` true _output)
          (set `/Game/Blueprints/MotionControllerPawn2.DatapointPointedAt` null _output))))))

(event `/Game/VirtualRealityBP/Blueprints/ResizeActorInterface.StartScan`
  ;[1 1 1] Scanning Feature
  (if (and (!= (`self.ScannerCoverObject`) null) (`/Game/Blueprints/EROS_GameInstance.bDataPointsUnlocked` (`self.GIRef`)))
    (bind _returnvalue (`KismetSystemLibrary.K2_SetTimerDelegate` (delegate `HandleScannerTimer`) 1.75))
    (set `self.ScanningTimerHandle` _returnvalue)
    (`AudioComponent.Play` (`self.ScannerLoop`) 0.0)
    (else
      (`/Game/Blueprints/MotionControllerPawn2.ShowNotification` (`self.CharRef`) "<- DataPoints not unlocked ->" (struct :`R` 1.0 :`B` 0.781225 :`A` 1.0)))))

(event `HandleScannerTimer`
  ;[1 1 1] Scanning Feature
  (`self.ScanSuccessful`)
  (`AudioComponent.Stop` (`self.ScannerLoop`)))

(event `/Game/VirtualRealityBP/Blueprints/ResizeActorInterface.EndScan`
  ;[1 1 1] Scanning Feature
  (`KismetSystemLibrary.K2_ClearAndInvalidateTimerHandle` (`self.ScanningTimerHandle`))
  (`AudioComponent.Stop` (`self.ScannerLoop`)))

(event `ScanSuccessful`
  ;[1 1 1] Scanning Feature
  (`ActorComponent.K2_DestroyComponent` (`self.ScannerCoverObject`))
  (`GameplayStatics.PlaySound2D` "/Game/Sounds/Scan_Successful.Scan_Successful" 1.0 1.0 0.0 null null)
  (`KismetSystemLibrary.K2_ClearAndInvalidateTimerHandle` (`self.RockPulseTimerHandle`))
  (`self.RevealAnimation`)
  (`self.UpdateSaveInformation`))

(event `RevealAnimation`
  (bind _pillarmesh (`self.PillarMesh`))
  (bind (_pillarstartlocation_x _pillarstartlocation_y _pillarstartlocation_z) (`KismetMathLibrary.BreakVector` (`self.PillarStartLocation`)))
  ;[1 1 1] Scanner Reveal Animation
  (`SceneComponent.SetVisibility` _pillarmesh true false)
  (bind (_direction _newtrack_0) (`Timeline|ScannerRevealLocation`)
    (:`Update`
      (`SceneComponent.K2_SetWorldLocation` _pillarmesh (`KismetMathLibrary.VLerp` (`self.PillarStartLocation`) (`KismetMathLibrary.MakeVector` _pillarstartlocation_x _pillarstartlocation_y (+ _pillarstartlocation_z 150.0)) _newtrack_0) false false))
    (:`Finished`
      (`KismetSystemLibrary.Delay` 1.5)
      (bind (_direction_2 _newtrack_0_2) (`Timeline|ScannerRevealRotation`)
        (:`Update`
          (`SceneComponent.K2_AddLocalRotation` (`self.PillarMesh`) (`KismetMathLibrary.MakeRotator` 0.0 0.0 (* _newtrack_0_2 (`self.RotationRate`))) false false))))))

(event `ToggleHandControls`
  ;[1 1 1] ToggleHandControls New
  (if (`self.bIsToggleComplete`)
    (set `self.bIsToggleComplete` false)
    (`/Engine/EditorBlueprintResources/StandardMacros.FlipFlop`
      (:`A`
        (bind (_direction _newtrack_0) (`Timeline|Temp` :!via `PlayFromStart` :!label _label_2)
          (:`Update`
            (`self.SetupButtonDest` _newtrack_0 (`self.RightButton`) (`self.EndPoint1`))
            (`self.SetupButtonDest` _newtrack_0 (`self.LeftButton`) (`self.EndPoint3`)))
          (:`Finished`
            (`KismetSystemLibrary.Delay` 0.5)
            (set `self.bIsToggleComplete` true))))
      (:`B`
        (goto _label_2 :!via `ReverseFromEnd`)))))

(event `HandButtonAnimation`
  (params (bIsStartingPress :type Boolean))
  ;[1 1 1] HandButtonAnimation
)

(event `self.RightButton.OnComponentEndOverlap`
  (params (OverlappedComponent :type "PrimitiveComponent Object Reference") (OtherActor :type "Actor Object Reference") (OtherComp :type "PrimitiveComponent Object Reference") (OtherBodyIndex :type Integer))
  ;[1 1 1] end overlap, unused at the moment
  (bind _outactors (`GameplayStatics.GetAllActorsOfClass` "/Game/Blueprints/MotionControllerPawn2.MotionControllerPawn2_C"))
  (bind _output (`|GetArrayItem` _outactors))
  (if (or (== (`/Game/Blueprints/Character/BP_MotionController2.GrabSphere` (`/Game/Blueprints/MotionControllerPawn2.RController` _output)) OtherComp) (== (`/Game/Blueprints/Character/BP_MotionController2.GrabSphere` (`/Game/Blueprints/MotionControllerPawn2.LController` _output)) OtherComp))
    _))

(event `self.RightButton.OnComponentBeginOverlap`
  (params (OverlappedComponent :type "PrimitiveComponent Object Reference") (OtherActor :type "Actor Object Reference") (OtherComp :type "PrimitiveComponent Object Reference") (OtherBodyIndex :type Integer) (bFromSweep :type Boolean) (SweepResult :type "HitResult Structure (by ref)"))
  ;[1 1 1] Overlapping hand controllers with hand buttons
  (set `self.CurrentButtonPressed` (`self.RightButton`))
  (bind _bishandoverlapping (`self.ProcessButtonPress` OtherComp))
  (if _bishandoverlapping
    (if (`self.bIsToggleComplete`)
      (set `self.MoveInvert` 1)
      (`self.StartRButtonAction`))))

(event `self.RSphereInner.OnComponentBeginOverlap`
  (params (OverlappedComponent :type "PrimitiveComponent Object Reference") (OtherActor :type "Actor Object Reference") (OtherComp :type "PrimitiveComponent Object Reference") (OtherBodyIndex :type Integer) (bFromSweep :type Boolean) (SweepResult :type "HitResult Structure (by ref)"))
  ;[1 1 1] maybe use with hand button animation.
)

(event `self.RSphere.OnComponentEndOverlap`
  (params (OverlappedComponent :type "PrimitiveComponent Object Reference") (OtherActor :type "Actor Object Reference") (OtherComp :type "PrimitiveComponent Object Reference") (OtherBodyIndex :type Integer))
  ;[1 1 1] maybe use with hand button animation.
)

(event `self.LeftButton.OnComponentEndOverlap`
  (params (OverlappedComponent :type "PrimitiveComponent Object Reference") (OtherActor :type "Actor Object Reference") (OtherComp :type "PrimitiveComponent Object Reference") (OtherBodyIndex :type Integer))
  ;[1 1 1] end overlap, unused at the moment
)

(event `self.LeftButton.OnComponentBeginOverlap`
  (params (OverlappedComponent :type "PrimitiveComponent Object Reference") (OtherActor :type "Actor Object Reference") (OtherComp :type "PrimitiveComponent Object Reference") (OtherBodyIndex :type Integer) (bFromSweep :type Boolean) (SweepResult :type "HitResult Structure (by ref)"))
  ;[1 1 1] Overlapping hand controllers with hand buttons
  (set `self.CurrentButtonPressed` (`self.LeftButton`))
  (bind _bishandoverlapping (`self.ProcessButtonPress` OtherComp))
  (if _bishandoverlapping
    (if (`self.bIsToggleComplete`)
      (set `self.MoveInvert` 1)
      (`self.StartLButtonAction`))))

(event `self.Sphere.OnComponentBeginOverlap`
  (params (OverlappedComponent :type "PrimitiveComponent Object Reference") (OtherActor :type "Actor Object Reference") (OtherComp :type "PrimitiveComponent Object Reference") (OtherBodyIndex :type Integer) (bFromSweep :type Boolean) (SweepResult :type "HitResult Structure (by ref)"))
  (bind _bishandoverlapping (`self.ProcessButtonPress` OtherComp))
  (if _bishandoverlapping
    (if (and (`self.bIsToggleComplete`) (`self.bIsInactive`))
      (`self.ToggleTextVisibility` true)
      (`self.StartPedestalButtonPress`)
      (set `self.bIsInactive` false))))

(event `self.PillarMesh.OnComponentBeginOverlap`
  (params (OverlappedComponent :type "PrimitiveComponent Object Reference") (OtherActor :type "Actor Object Reference") (OtherComp :type "PrimitiveComponent Object Reference") (OtherBodyIndex :type Integer) (bFromSweep :type Boolean) (SweepResult :type "HitResult Structure (by ref)")))

(event `ToggleTextVisibility`
  (params (bIsTurningOn :type Boolean))
  (`SceneComponent.SetVisibility` (`self.RightButtonText`) bIsTurningOn false)
  (`SceneComponent.SetVisibility` (`self.LeftButtonText`) bIsTurningOn false))

(fn `BoxOverlapFunction`)

(fn `ChildBeginPlay`)

(fn `EndLButtonAction`)

(fn `EndRButtonAction`)

(fn `ProcessButtonPress`
  (params (InputPin :type "Object Object Reference"))
  (returns (bIsHandOverlapping :type Boolean))
  (bind _outactors (`GameplayStatics.GetAllActorsOfClass` "/Game/Blueprints/MotionControllerPawn2.MotionControllerPawn2_C"))
  (bind _output (`|GetArrayItem` _outactors))
  (if (== (`/Game/Blueprints/Character/BP_MotionController2.GrabSphere` (`/Game/Blueprints/MotionControllerPawn2.RController` _output)) InputPin)
    _
    (elif (== (`/Game/Blueprints/Character/BP_MotionController2.GrabSphere` (`/Game/Blueprints/MotionControllerPawn2.LController` _output)) InputPin)
      _
      (else
        (return false))))
  (set `/Game/Blueprints/MotionControllerPawn2.bIsPointingAtScanObject` true _output)
  (return true))

(fn `SetupButtonDest`
  (params (Alpha :type "Float (double-precision)") (ButtonToMove :type "SceneComponent Object Reference") (WhichEndpoint :type "SceneComponent Object Reference"))
  (`SceneComponent.K2_SetWorldLocation` ButtonToMove (`KismetMathLibrary.VLerp` (`SceneComponent.K2_GetComponentLocation` (`self.StartingPoint`)) (`SceneComponent.K2_GetComponentLocation` WhichEndpoint) Alpha) false false))

(fn `StartLButtonAction`)

(fn `StartPedestalButtonPress`)

(fn `StartRButtonAction`)

(fn `UserConstructionScript`
  (`TextRenderComponent.K2_SetText` (`self.RightButtonText`) (`self.RButtonText`))
  (`TextRenderComponent.K2_SetText` (`self.LeftButtonText`) (`self.LButtonText`))
  (set `self.PillarStartLocation` (`SceneComponent.K2_GetComponentLocation` (`self.PillarMesh`))))

(fn `WhatsMyName`
  (returns (Output_Get :type Text))
  (bind _output_get (set `self.MyName` (`KismetTextLibrary.Conv_StringToText` (`KismetStringLibrary.Concat_StrStr` (`KismetSystemLibrary.GetDisplayName` self) " Gallery Object Unlocked"))))
  (return _output_get))