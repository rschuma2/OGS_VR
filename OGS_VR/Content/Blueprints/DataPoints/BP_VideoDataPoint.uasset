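; BP_VideoDataPoint is a child data point actor that plays a video on a widget, operated with motion controller hand buttons.
; Player overlap hands its video and itself to the game instance reference, and the pedestal press activates the widget and reveals the buttons.
; Inherited buttons play and restart the video, while an added third button deactivates the data point.
; An overridden timeline toggle animates all three buttons, gated against re-triggering mid-move.
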(event `self.ReceiveBeginPlay`
  ;[1 1 1] BeginPlay
  (`parent.ReceiveBeginPlay`))

(event `self.ChildBeginPlay`
  ;[1 1 1] BeginPlay
  (bind _asw_video_data_point (cast `/Game/NasaEROSVR/UI/W_VideoDataPoint` (`WidgetComponent.GetUserWidgetObject` (`self.Widget`))))
  (set `self.ThisWidget` _asw_video_data_point))

(event `self.ReceiveActorBeginOverlap`
  (params (OtherActor :type "Actor Object Reference"))
  ;[1 1 1] set up datapoint on player overlap
  (cast `/Game/Blueprints/MotionControllerPawn2` OtherActor)
  (set `/Game/Blueprints/EROS_GameInstance.MediaSourceToPlay` (`self.VideoToPlay`) (`self.GIRef`))
  (set `/Game/Blueprints/EROS_GameInstance.CurrentVideoatapoint` self (`self.GIRef`)))

(event `self.Button3.OnComponentBeginOverlap`
  (params (OverlappedComponent :type "PrimitiveComponent Object Reference") (OtherActor :type "Actor Object Reference") (OtherComp :type "PrimitiveComponent Object Reference") (OtherBodyIndex :type Integer) (bFromSweep :type Boolean) (SweepResult :type "HitResult Structure (by ref)"))
  ;[1 1 1] New Hand Control overlap check. same as parent for first two controls.
  (set `self.CurrentButtonPressed` (`self.Button3`))
  (bind _bishandoverlapping (`self.ProcessButtonPress` OtherComp))
  (if _bishandoverlapping
    (set `self.MoveInvert` 1)
    (`self.ButtonThreeAction`)))

(event `self.StartPedestalButtonPress`
  (set `self.ZFlip` 3.2)
  (set `self.XYFlip` -5.0)
  (`self.ToggleHandControls`)
  (`/Game/NasaEROSVR/UI/W_VideoDataPoint.ActivateDatapoint` (`self.ThisWidget`)))

(event `self.StartRButtonAction`
  ;[1 1 1] Hand Control Actions
  (`GameplayStatics.PlaySound2D` "/Game/NasaEROSVR/Sounds/MinimalUI/370846__cabled-mess__funny-click-minimal-ui-sounds.370846__cabled-mess__funny-click-minimal-ui-sounds" 1.0 1.0 0.0 null null)
  (`/Game/NasaEROSVR/UI/W_VideoDataPoint.PlayVideo` (`self.ThisWidget`)))

(event `self.StartLButtonAction`
  ;[1 1 1] Hand Control Actions
  (`GameplayStatics.PlaySound2D` "/Game/NasaEROSVR/Sounds/MinimalUI/370846__cabled-mess__funny-click-minimal-ui-sounds.370846__cabled-mess__funny-click-minimal-ui-sounds" 1.0 1.0 0.0 null null)
  (`/Game/NasaEROSVR/UI/W_VideoDataPoint.RestartVideo` (`self.ThisWidget`)))

(event `ButtonThreeAction`
  ;[1 1 1] Hand Control Actions
  (`GameplayStatics.PlaySound2D` "/Game/NasaEROSVR/Sounds/MinimalUI/370846__cabled-mess__funny-click-minimal-ui-sounds.370846__cabled-mess__funny-click-minimal-ui-sounds" 1.0 1.0 0.0 null null)
  (if (`self.bIsToggleComplete`)
    (set `self.ZFlip` -3.2)
    (set `self.XYFlip` 5.0)
    (`self.ToggleHandControls`)
    (`/Game/NasaEROSVR/UI/W_VideoDataPoint.DeactivateDatapoint` (`self.ThisWidget`))
    (`KismetSystemLibrary.Delay` 2.0)
    (set `self.bIsInactive` true)))

(event `self.ToggleHandControls`
  ;[1 1 1] Toggle Hand Controls (Overridden to include extra button)
  (if (`self.bIsToggleComplete`)
    (set `self.bIsToggleComplete` false)
    (`/Engine/EditorBlueprintResources/StandardMacros.FlipFlop`
      (:`A`
        (bind (_direction _newtrack_0) (`Timeline|Timeline_0` :!via `PlayFromStart` :!label _label)
          (:`Update`
            (`self.SetupButtonDest` _newtrack_0 (`self.RightButton`) (`self.EndPoint2`))
            (`self.SetupButtonDest` _newtrack_0 (`self.LeftButton`) (`self.EndPoint1`))
            (`self.SetupButtonDest` _newtrack_0 (`self.Button3`) (`self.EndPoint3`)))
          (:`Finished`
            (`KismetSystemLibrary.Delay` 0.5)
            (set `self.bIsToggleComplete` true))))
      (:`B`
        (goto _label :!via `ReverseFromEnd`)))))

(fn `UserConstructionScript`
  (`parent.UserConstructionScript`))