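; EROS game instance, the shared hub for menus, scene transitions, level streaming, saves and solar system settings.
; Show events lazily create cached widgets, and most freeze time via global dilation for UI-only input until RemoveMenu resumes play.
; DT_SceneTransitions rows feed transition info, while streaming swaps levels and repositions the pawn.
; SaveSlot records level progress and countdown completion, but LoadGame's cast is unwired, so loaded data is never applied.
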(event `SetupGameInputMode`
  (bind _returnvalue (`GameplayStatics.GetPlayerController` 0))
  ;[1 1 1] FPSCharacter testing only.
  ;;[1 1 1] SetupGameInputMode - resume time and set input to game mode. hide mouse cursor
  (`WidgetBlueprintLibrary.SetInputMode_GameOnly` _returnvalue)
  (set `PlayerController.bShowMouseCursor` false _returnvalue)
  (`GameplayStatics.SetGlobalTimeDilation` 1.0))

(event `ShowMainMenu`
  ;[1 1 1] ShowMainMenu - If not valid, first creates menu; then adds it to the viewport.
  (`/Engine/EditorBlueprintResources/StandardMacros.IsValid` (`self.MainMenuWidget`)
    (:`Is Valid`
      _)
    (:`Is Not Valid`
      (bind _returnvalue (`|CreateWidget` "/Game/NasaEROSVR/UI/W_MainMenu.W_MainMenu_C"))
      (bind _output_get (set `self.MainMenuWidget` _returnvalue))))
  (`UserWidget.AddToViewport` _output_get 0)
  (`self.SetupMenuInputMode`))

(event `SetupMenuInputMode`
  (bind _returnvalue (`GameplayStatics.GetPlayerController` 0))
  ;[1 1 1] FPSCharacter testing only.
  ;;[1 1 1] SetupMenuInputMode - stop time and set input to menu mode. show mouse cursor.
  (`GameplayStatics.SetGlobalTimeDilation` 0.0)
  (`WidgetBlueprintLibrary.SetInputMode_UIOnlyEx` _returnvalue (`self.CurrentDataPointWidget`))
  (set `PlayerController.bShowMouseCursor` true _returnvalue))

(event `ShowTransitionScreen`
  (bind _returnvalue (`GameplayStatics.GetPlayerController` 0))
  ;[1 1 1] ShowSceneTransition
  (`/Engine/EditorBlueprintResources/StandardMacros.IsValid` (`self.WSceneTransition`)
    (:`Is Valid`
      _)
    (:`Is Not Valid`
      (bind _returnvalue_2 (`|CreateWidget` "/Game/NasaEROSVR/UI/W_SceneTransition.W_SceneTransition_C"))
      (set `self.WSceneTransition` _returnvalue_2)))
  (`UserWidget.AddToViewport` (`self.WSceneTransition`) 0)
  (`WidgetBlueprintLibrary.SetInputMode_UIOnlyEx` _returnvalue null)
  (set `PlayerController.bShowMouseCursor` true _returnvalue))

(event `ShowScannerWidget`
  (params (SoundToPlay :type "SoundBase Object Reference") (WidgetToLoad :type "UserWidget Class Reference"))
  ;[1 1 1] ShowScannerWidget
  (`/Engine/EditorBlueprintResources/StandardMacros.IsValid` (`self.CurrentScannerWidget`)
    (:`Is Valid`
      _)
    (:`Is Not Valid`
      (bind _returnvalue (`|CreateWidget` WidgetToLoad (`GameplayStatics.GetPlayerController` 0)))
      (bind _output_get (set `self.CurrentScannerWidget` _returnvalue))))
  (`UserWidget.AddToViewport` _output_get 0)
  (`GameplayStatics.PlaySound2D` SoundToPlay 1.0 1.0 0.0 null null)
  (`self.SetupMenuInputMode`))

(event `ShowDataPoint`
  (params (WidgetToLoad :type "UserWidget Class Reference") (SoundToPlay :type "SoundBase Object Reference"))
  ;[1 1 1] ShowDataPoint - Shows the appropriate data point widget. Updated by DataPoint bp based on instance editable var.
  (`/Engine/EditorBlueprintResources/StandardMacros.IsValid` (`self.CurrentDataPointWidget`)
    (:`Is Valid`
      _)
    (:`Is Not Valid`
      (bind _returnvalue (`|CreateWidget` WidgetToLoad (`GameplayStatics.GetPlayerController` 0)))
      (bind _output_get (set `self.CurrentDataPointWidget` _returnvalue))))
  (`UserWidget.AddToViewport` _output_get 0)
  (`GameplayStatics.PlaySound2D` SoundToPlay 1.0 1.0 0.0 null null)
  (`self.SetupMenuInputMode`))

(event `StartCountdownTimer`
  (params (CurrentLevelDuration :type Integer))
  ;[1 1 1] DevTool UITest CountdownTimer
  (set `self.TestWidgetCountdownTimer` CurrentLevelDuration)
  (bind _returnvalue (`KismetSystemLibrary.K2_SetTimerDelegate` (delegate `HandleCountdownTimer`) 1.0 true))
  (set `self.CountdownTimerHandle` _returnvalue))

(event `RemoveMenu`
  (params (WidgetToRemove :type "UserWidget Object Reference") (SoundToPlay :type "SoundBase Object Reference"))
  (bind _returnvalue (`GameplayStatics.GetPlayerController` 0))
  ;[1 1 1] RemoveMenu - Remove specified menu from Viewport. May not want this for world space widgets, and will not want to adjust mouse cursor or maybe input mode with motion controller pawn.
  (`Widget.RemoveFromParent` WidgetToRemove)
  (`WidgetBlueprintLibrary.SetInputMode_GameOnly` _returnvalue)
  (set `PlayerController.bShowMouseCursor` false _returnvalue)
  (`GameplayStatics.PlaySound2D` SoundToPlay 1.0 1.0 0.0 null null)
  (`self.SetupGameInputMode`))

(event `HandleCountdownTimer`
  (bind (_savedata_testvalue _savedata_currentlevel _savedata_bislocomotionactive) (break `/Game/Blueprints/Data/SaveSystemStruct` (`/Game/Blueprints/SaveSystem/EROSSave.SaveData` (`self.ErosGameSave`))))
  ;[1 1 1] DevTool UITest CountdownTimer
  (bind _output_get (set `self.TestWidgetCountdownTimer` (`KismetMathLibrary.Clamp` (- (`self.TestWidgetCountdownTimer`) 1) 0 (stale `StartCountdownTimer` CurrentLevelDuration))))
  (if (<= _output_get 0)
    (`KismetSystemLibrary.K2_ClearAndInvalidateTimerHandle` (`self.CountdownTimerHandle`))
    (`self.CheckForSave`)
    (set `/Game/Blueprints/SaveSystem/EROSSave.SaveData` (make `/Game/Blueprints/Data/SaveSystemStruct` _savedata_testvalue _savedata_currentlevel _savedata_bislocomotionactive true) (`self.ErosGameSave`))
    (`self.SaveGame`)))

(event `CheckRefs`
  ;[1 0 0.8462] CheckRefs ALWAYS DO THIS
  (`self.CharRef`
    (:`then`)
    (:`else`
      (bind _asmotion_controller_pawn_2 (cast `/Game/Blueprints/MotionControllerPawn2` (`GameplayStatics.GetPlayerCharacter` 0)))
      (set `self.CharRef` _asmotion_controller_pawn_2))))

(event `SetupSceneTransition`
  (params (RowName :type Name))
  (bind (_savedata_testvalue _savedata_currentlevel _savedata_bislocomotionactive _savedata_bislevelcomplete) (break `/Game/Blueprints/Data/SaveSystemStruct` (`/Game/Blueprints/SaveSystem/EROSSave.SaveData` (`self.ErosGameSave`))))
  ;[1 1 1] Setup Scene Transition
  (if (!= RowName "None")
    (bind _returnvalue (`|GetDataTableRow` "/Game/Blueprints/Data/DT_SceneTransitions.DT_SceneTransitions" RowName)
      (:`then`
        (bind _output_get (set `self.CurrentSceneTransitionInfo` _returnvalue))
        (set `self.NextLevelName` (`.NextLevelName_41_7A21B400475AA99C4F7AC190C5AFB716` (break `/Game/Blueprints/Data/Struct_SceneTransitions` _output_get)))))
    (else
      (bind _returnvalue_2 (`GameplayStatics.GetCurrentLevelName` true))
      (bind _returnvalue_3 (`KismetStringLibrary.Conv_StringToName` _returnvalue_2))
      (bind _returnvalue_4 (`|GetDataTableRow` "/Game/Blueprints/Data/DT_SceneTransitions.DT_SceneTransitions" _returnvalue_3)
        (:`then`
          (set `self.CurrentSceneTransitionInfo` _returnvalue_4)
          ;[1 1 1] testing save game setup. This might load the wrong level; need to check agaisnt Data table
          (`self.CheckForSave`)
          (set `/Game/Blueprints/SaveSystem/EROSSave.SaveData` (make `/Game/Blueprints/Data/SaveSystemStruct` _savedata_testvalue _returnvalue_3 _savedata_bislocomotionactive _savedata_bislevelcomplete) (`self.ErosGameSave`))
          (`self.SaveGame`))))))

(event `PlaySceneMusic`
  ;[1 1 1] PlaySceneMusic -> Play standard set of ambient sounds / music
  (`GameplayStatics.PlaySound2D` "/Game/NasaEROSVR/Sounds/246154__lerwickdj__16-ca-pads.246154__lerwickdj__16-ca-pads" 0.2 1.0 0.0 null null)
  (`GameplayStatics.PlaySound2D` "/Game/NasaEROSVR/Sounds/39628__anicator__sci-fi-ambient-01.39628__anicator__sci-fi-ambient-01" 0.2 1.0 0.0 null null)
  (`GameplayStatics.PlaySound2D` "/Game/NasaEROSVR/Sounds/468407__onderwish__sci-fi-survival-dreamscape__1_.468407__onderwish__sci-fi-survival-dreamscape__1_" 0.5 1.0 0.0 null null))

(event `SaveGame`
  ;[1 1 1] SaveSystem
  ;;[1 1 1] SaveGame Event
  (`/Engine/EditorBlueprintResources/StandardMacros.IsValid` (`self.ErosGameSave`)
    (:`Is Valid`
      _)
    (:`Is Not Valid`
      (bind _returnvalue (`GameplayStatics.CreateSaveGameObject` "/Game/Blueprints/SaveSystem/EROSSave.EROSSave_C"))
      (set `self.ErosGameSave` _returnvalue)))
  (`GameplayStatics.SaveGameToSlot` (`self.ErosGameSave`) "SaveSlot"))

(event `TempResetLevelVariables`
  (params (TestNumDataPoints :type Integer) (TestNumGalleryItems :type Integer))
  ;[1 1 1] Temp Reset Level Variables
  (set `self.TestDataPointsFound` 0)
  (set `self.TestGalleryItemsFound` 0)
  (set `self.TestNumDataPoints` TestNumDataPoints)
  (set `self.TestNumGalleryItems` TestNumGalleryItems))

(event `CheckForSave`
  ;[1 1 1] SaveSystem
  ;;[1 1 1] CheckForSave Event
  (`/Engine/EditorBlueprintResources/StandardMacros.IsValid` (`self.ErosGameSave`)
    (:`Is Not Valid`
      (bind _returnvalue (`GameplayStatics.CreateSaveGameObject` "/Game/Blueprints/SaveSystem/EROSSave.EROSSave_C"))
      (set `self.ErosGameSave` _returnvalue))))

(event `SetupSolarSystem`
  (params (Scale :type "Float (double-precision)") (PlayRate :type "Float (double-precision)") (IsMoving :type Boolean) (CameraToFollow :type "CameraActor Object Reference") (StartDate :type "/Game/Blueprints/Data/StructSpaceBodyInfo Structure") (EndDate :type "/Game/Blueprints/Data/StructSpaceBodyInfo Structure") (`Space Body Info Is Looping` :type Boolean))
  ;[1 1 1] SetupSolarSystem
  (set `self.SolarSystemScale` Scale)
  (set `self.SpaceBodyInfo` (make `/Game/Blueprints/Data/SpaceBodyStruct` PlayRate IsMoving CameraToFollow StartDate EndDate `Space Body Info Is Looping`)))

(event `LoadGame`
  ;[1 1 1] SaveSystem
  (`self.CheckRefs`)
  (`self.CheckForSave`)
  (bind _returnvalue (`GameplayStatics.LoadGameFromSlot` "SaveSlot"))
  (`/Game/Blueprints/MotionControllerPawn2.UpdateUnlocks` (`self.CharRef`))
  (`self.UpdateUnlocks`))

(event `UpdateUnlocks`
  (bind (_featureunlocks_grip _featureunlocks_jump _featureunlocks_galleryscene _featureunlocks_solarsystemscene _featureunlocks_resize _featureunlocks_scanner _featureunlocks_datapoints _featureunlocks_galleryitems _featureunlocks_sceneselection) (break `/Game/Blueprints/Data/FeatureUnlockStruct` (`/Game/Blueprints/SaveSystem/EROSSave.FeatureUnlocks` (`self.ErosGameSave`))))
  ;[1 1 1] Update Unlocks
  (set `self.bGalleryMapUnlocked` _featureunlocks_galleryscene)
  (set `self.bSolarSystemUnlocked` _featureunlocks_solarsystemscene)
  (set `self.bDataPointsUnlocked` _featureunlocks_datapoints)
  (set `self.bGalleryObjectsUnlocked` _featureunlocks_galleryitems)
  (set `self.bSceneSelectionUnlocked` _featureunlocks_sceneselection))

(event `MyLevelStream`
  (params (LevelToLoad :type Name) (LevelToUnload :type Name) (NewTransform :type "Transform Structure") (LoadTime :type "Float (double-precision)"))
  (bind _charref (`self.CharRef`))
  ;[1 1 1] HandleLevelStreaming
  (`self.CheckRefs`)
  (`GameplayStatics.LoadStreamLevel` LevelToLoad true)
  (`GameplayStatics.UnloadStreamLevel` LevelToUnload)
  (if (`/Game/Blueprints/MotionControllerPawn2.bIsUnloaded` _charref)
    _
    (else
      _))
  (`/Game/Blueprints/MotionControllerPawn2.WorldUnloadLoad` _charref false)
  (`Actor.K2_SetActorTransform` (`self.CharRef`) NewTransform false false))

(fn `GetSceneTransitionInfo`
  (returns (SceneDate :type Text) (DaysTill :type Text) (NEARLoc :type Text) (ErosLoc :type Text) (MapLoc :type Text) (MapDFromPrev :type Text) (POI1 :type Text) (POI2 :type Text) (MapImg :type "SlateBrush Structure") (NextLevel :type Text))
  (bind (_currentscenetransitioninfo_name _currentscenetransitioninfo_datemonthddyyyy _currentscenetransitioninfo_daystillneararrivaloneros _currentscenetransitioninfo_neardistfromeros _currentscenetransitioninfo_erosdistfromearth _currentscenetransitioninfo_locationoneros _currentscenetransitioninfo_distfromlastposkm _currentscenetransitioninfo_pointofinterest1 _currentscenetransitioninfo_pointofinterest2 _currentscenetransitioninfo_mapimg _currentscenetransitioninfo_nextlevelname) (break `/Game/Blueprints/Data/Struct_SceneTransitions` (`self.CurrentSceneTransitionInfo`)))
  (return _currentscenetransitioninfo_datemonthddyyyy _currentscenetransitioninfo_daystillneararrivaloneros _currentscenetransitioninfo_neardistfromeros _currentscenetransitioninfo_erosdistfromearth _currentscenetransitioninfo_locationoneros _currentscenetransitioninfo_distfromlastposkm _currentscenetransitioninfo_pointofinterest1 _currentscenetransitioninfo_pointofinterest2 _currentscenetransitioninfo_mapimg (`KismetTextLibrary.Conv_NameToText` _currentscenetransitioninfo_nextlevelname)))