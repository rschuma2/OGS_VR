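; BP_GalleryItem2 is a gallery mode item that the motion controller can pick up and drop, with its placement saved.
; The construction script applies mesh and material from its SaveInfo struct.
; Pickup plays a sound and attaches the item; Drop detaches it, waits briefly, then records the new transform.
; Saving matches entries in the game instance's save by mesh, overwriting a match or appending a new one.
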(event `self.ReceiveBeginPlay`
  (bind _aseros_game_instance (cast `/Game/Blueprints/EROS_GameInstance` (`GameplayStatics.GetGameInstance`)))
  (set `self.GIRef` _aseros_game_instance))

(event `/Game/Blueprints/Character/PickupActorInterface.Pickup`
  (params (AttachTo :type "SceneComponent Object Reference"))
  (`GameplayStatics.SpawnSoundAttached` "/Game/NasaEROSVR/Sounds/plastic_pickup_Cue.plastic_pickup_Cue" (`self.DefaultSceneRoot`) "None" (0.0 0.0 0.0) (struct) "KeepRelativeOffset" false 1.0 1.0 0.0 null null)
  (`SceneComponent.K2_AttachToComponent` (`self.K2_GetRootComponent`) AttachTo "None" "KeepWorld" "KeepWorld" "KeepWorld" false))

(event `UpdateSaveInformation`
  (bind _giref (`self.GIRef`))
  (bind (_saveinfo_bisunlocked _saveinfo_currenttransform _saveinfo_currentmesh) (break `/Game/Blueprints/Data/GaleryItemsStruct` (`self.SaveInfo`)))
  (bind (_saveinfo_bisunlocked_2 _saveinfo_currenttransform_2 _saveinfo_currentmesh_2) (break `/Game/Blueprints/Data/GaleryItemsStruct` (`self.SaveInfo`)))
  (bind (_saveinfo_bisunlocked_3 _saveinfo_currenttransform_3 _saveinfo_currentmesh_3 _saveinfo_currentmaterial _saveinfo_displayedon) (break `/Game/Blueprints/Data/GaleryItemsStruct` (`self.SaveInfo`)))
  (bind (_saveinfo_bisunlocked_4 _saveinfo_currenttransform_4 _saveinfo_currentmesh_4) (break `/Game/Blueprints/Data/GaleryItemsStruct` (`self.SaveInfo`)))
  (bind _galleryitems (`/Game/Blueprints/SaveSystem/EROSSave.GalleryItems` (`/Game/Blueprints/EROS_GameInstance.ErosGameSave` _giref)))
  (`/Game/Blueprints/EROS_GameInstance.CheckForSave` _giref)
  (for (_array_element _array_index) _galleryitems
    (bind _output_get (set `self.CurrentElement` _array_element))
    ;[1 1 1] Update info if found
    (if (== (`.CurrentMesh_17_3D053CBF466E9965224C27AF86515FAB` (break `/Game/Blueprints/Data/GaleryItemsStruct` _output_get)) _saveinfo_currentmesh_2)
      (set `self.bFoundMatch` true)
      (bind _output_get_2 (set `self.CurrentElement` (make `/Game/Blueprints/Data/GaleryItemsStruct` _saveinfo_bisunlocked_3 _saveinfo_currenttransform_3 _saveinfo_currentmesh_3 _saveinfo_currentmaterial _saveinfo_displayedon)))
      (`KismetArrayLibrary.Array_Set` (`/Game/Blueprints/SaveSystem/EROSSave.GalleryItems` (`/Game/Blueprints/EROS_GameInstance.ErosGameSave` (`self.GIRef`))) _array_index _output_get_2)
      (`/Game/Blueprints/EROS_GameInstance.SaveGameTest` (`self.GIRef`))
      (`KismetSystemLibrary.PrintString` (`KismetSystemLibrary.GetDisplayName` _saveinfo_currentmesh) true true (struct :`G` 1.0 :`B` 0.183741 :`A` 1.0))
      (break)))
  ;[1 1 1] Add item if not found
  (if (not (`self.bFoundMatch`))
    (bind _returnvalue (`KismetArrayLibrary.Array_Add` _galleryitems (`self.SaveInfo`)))
    (set `self.MySaveStructArrayIndex` _returnvalue)
    (`/Game/Blueprints/EROS_GameInstance.SaveGameTest` (`self.GIRef`))
    (`KismetSystemLibrary.PrintString` (`KismetStringLibrary.Concat_StrStr` "new item: " (`KismetSystemLibrary.GetDisplayName` _saveinfo_currentmesh_4)))))

(event `/Game/Blueprints/Character/PickupActorInterface.Drop`
  (bind (_saveinfo_bisunlocked _saveinfo_currenttransform _saveinfo_currentmesh _saveinfo_currentmaterial _saveinfo_displayedon) (break `/Game/Blueprints/Data/GaleryItemsStruct` (`self.SaveInfo`)))
  (`self.K2_DetachFromActor` "KeepWorld" "KeepWorld" "KeepWorld")
  (`KismetSystemLibrary.Delay` 0.2)
  (set `self.SaveInfo` (make `/Game/Blueprints/Data/GaleryItemsStruct` _saveinfo_bisunlocked (`self.GetTransform` self) _saveinfo_currentmesh _saveinfo_currentmaterial _saveinfo_displayedon))
  (`self.UpdateSaveInformation`))

(fn `UserConstructionScript`
  (bind (_saveinfo_bisunlocked _saveinfo_currenttransform _saveinfo_currentmesh _saveinfo_currentmaterial) (break `/Game/Blueprints/Data/GaleryItemsStruct` (`self.SaveInfo`)))
  (bind _staticmesh (`self.StaticMesh`))
  (`parent.UserConstructionScript`)
  (`StaticMeshComponent.SetStaticMesh` _staticmesh _saveinfo_currentmesh)
  (`PrimitiveComponent.SetMaterial` _staticmesh 0 _saveinfo_currentmaterial))