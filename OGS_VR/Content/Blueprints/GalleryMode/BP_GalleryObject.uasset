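; VR gallery collectible that players uncover by scanning, then grab, move and resize with two hands.
; Controller overlap marks it as the scan target; a short timed scan, gated by an unlock flag, destroys its cover and plays a rising reveal.
; The reveal updates or adds its save entry, notifying on new finds.
; Construction applies saved mesh and material; dropping in the Gallery level refreshes its transform and saves.
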(event `UpdateSaveInformation`
  (bind (_saveinfo_bisunlocked _saveinfo_currenttransform _saveinfo_currentmesh) (break `/Game/Blueprints/Data/GaleryItemsStruct` (`self.SaveInfo`)))
  (bind _giref (`self.GIRef`))
  (bind _giref_2 (`self.GIRef`))
  (bind (_output_numdatapoints _output_numgalleryitems _output_datapointsfound _output_galleryitemsfound) (break `/Game/Blueprints/Data/Struct_LevelInfo` (`|GetArrayItem` (`/Game/Blueprints/SaveSystem/EROSSave.LevelInfo` (`/Game/Blueprints/EROS_GameInstance.ErosGameSave` _giref)) (`/Game/Blueprints/EROS_GameInstance.CurrentLevelIndex` _giref))))
  ;[0 0.9267 1] UpdateSaveInfo (clean up and remove print strings after testing)
  (`/Game/Blueprints/EROS_GameInstance.CheckForSave` _giref_2)
  (for (_array_element _array_index) (`/Game/Blueprints/SaveSystem/EROSSave.GalleryItems` (`/Game/Blueprints/EROS_GameInstance.ErosGameSave` _giref_2))
    (bind _output_get (set `self.CurrentElement` _array_element))
    (if (== (`.CurrentMesh_17_3D053CBF466E9965224C27AF86515FAB` (break `/Game/Blueprints/Data/GaleryItemsStruct` _output_get)) _saveinfo_currentmesh)
      (set `self.bFoundMatch` true)
      (bind _currentelement (`self.UpdateTransform`))
      (`KismetArrayLibrary.Array_Set` (`/Game/Blueprints/SaveSystem/EROSSave.GalleryItems` (`/Game/Blueprints/EROS_GameInstance.ErosGameSave` (`self.GIRef`))) _array_index (make `/Game/Blueprints/Data/GaleryItemsStruct` (break `/Game/Blueprints/Data/GaleryItemsStruct` _currentelement) "0.000000,0.000000,0.000000|0.000000,0.000000,0.000000|1.000000,1.000000,1.000000" (`.CurrentMesh_17_3D053CBF466E9965224C27AF86515FAB` (break `/Game/Blueprints/Data/GaleryItemsStruct` _currentelement)) (`.CurrentMaterial_13_DF1C5E724B4DAF4E4D7AF4ABBD092241` (break `/Game/Blueprints/Data/GaleryItemsStruct` _currentelement)) (`.DisplayedOn_16_6D48140B4928CF58E790ADBB00F96EC3` (break `/Game/Blueprints/Data/GaleryItemsStruct` _currentelement))))
      (`/Game/Blueprints/EROS_GameInstance.SaveGame` (`self.GIRef`))
      (break)))
  ;;[1 1 1] Add item if not found
  (if (not (`self.bFoundMatch`))
    (bind _returnvalue (`KismetArrayLibrary.Array_Add` (`/Game/Blueprints/SaveSystem/EROSSave.GalleryItems` (`/Game/Blueprints/EROS_GameInstance.ErosGameSave` (`self.GIRef`))) (`self.SaveInfo`)))
    (set `self.MySaveStructArrayIndex` _returnvalue)
    (`BlueprintSetLibrary.Set_Add` _output_galleryitemsfound self)
    (`/Engine/EditorBlueprintResources/StandardMacros.IncrementInt` (`/Game/Blueprints/EROS_GameInstance.TestGalleryItemsFound` (`self.GIRef`))
      (:`  `
        (`/Game/Blueprints/EROS_GameInstance.SaveGame` (`self.GIRef`))
        (bind _output_get_2 (`self.WhatsMyName`))
        (`/Game/Blueprints/MotionControllerPawn2.ShowNotification` (`self.CharRef`) _output_get_2 (struct :`R` 0.019177 :`G` 1.0 :`A` 1.0))))))

(event `self.ReceiveBeginPlay`
  ;[1 1 1] BeginPlay
  (bind _aseros_game_instance (cast `/Game/Blueprints/EROS_GameInstance` (`GameplayStatics.GetGameInstance`)))
  (set `self.GIRef` _aseros_game_instance)
  (bind _asmotion_controller_pawn_2 (cast `/Game/Blueprints/MotionControllerPawn2` (`GameplayStatics.GetPlayerCharacter` 0)))
  (set `self.CharRef` _asmotion_controller_pawn_2)
  (bind _returnvalue (`PrimitiveComponent.CreateDynamicMaterialInstance` (`self.ScannerCoverObject`) 0 null "None"))
  (set `self.DynaMat` _returnvalue))

(event `ScannerPulseTimer`
  ;[1 1 1] ScannerPulseTimer
  (`/Engine/EditorBlueprintResources/StandardMacros.FlipFlop`
    (:`A`
      (`PrimitiveComponent.SetMaterial` (`self.ScannerCoverObject`) 0 "/Game/Megascans/3D_Assets/California_Coastal_Rock_Assembly_00/California_Coastal_Rock_Assembly_00_inst.California_Coastal_Rock_Assembly_00_inst"))
    (:`B`
      (`PrimitiveComponent.SetMaterial` (`self.ScannerCoverObject`) 0 "/Engine/ArtTools/RenderToTexture/Materials/Debug/M_Emissive_Color_0-0-127.M_Emissive_Color_0-0-127"))))

(event `HandleScannerPulseTimer`
  ;[1 1 1] BeginPlay
  (`self.ScannerPulseTimer`))

(event `/Game/VirtualRealityBP/Blueprints/ResizeActorInterface.StartResize`
  (params (`3rdHand` :type "/Game/Blueprints/Character/BP_MotionController2 Object Reference") (`4thHand` :type "/Game/Blueprints/Character/BP_MotionController2 Object Reference"))
  ;[1 1 1] StartResize
  (bind _output_get (set `self.3rdhand` `3rdHand`))
  (bind _output_get_2 (set `self.4thHand` `4thHand`))
  (if (and (`/Game/Blueprints/Character/BP_MotionController2.bGrabbing` _output_get) (`/Game/Blueprints/Character/BP_MotionController2.bGrabbing` _output_get_2))
    (set `self.bIsResizing` true)
    (set `self.InitialDistance` (`KismetMathLibrary.Abs` (`KismetMathLibrary.VSize` (- (`SceneComponent.K2_GetComponentLocation` (`/Game/Blueprints/Character/BP_MotionController2.HandMesh` (`self.3rdhand`))) (`SceneComponent.K2_GetComponentLocation` (`/Game/Blueprints/Character/BP_MotionController2.HandMesh` (`self.4thHand`)))))))
    (set `self.InitialScale` (`SceneComponent.K2_GetComponentScale` (`self.StaticMesh`)))))

(event `self.ReceiveTick`
  (params (DeltaSeconds :type "Float (single-precision)"))
  ;[1 1 1] EventTick
  (if (`self.bIsResizing`)
    (`SceneComponent.SetWorldScale3D` (`self.StaticMesh`) (* (`self.InitialScale`) (/ (`KismetMathLibrary.Abs` (`KismetMathLibrary.VSize` (- (`SceneComponent.K2_GetComponentLocation` (`/Game/Blueprints/Character/BP_MotionController2.HandMesh` (`self.3rdhand`))) (`SceneComponent.K2_GetComponentLocation` (`/Game/Blueprints/Character/BP_MotionController2.HandMesh` (`self.4thHand`)))))) (`self.InitialDistance`))))))

(event `/Game/VirtualRealityBP/Blueprints/ResizeActorInterface.EndResize`
  ;[1 1 1] EndResize
  (set `self.bIsResizing` false))

(event `/Game/Blueprints/Character/PickupActorInterface.Pickup`
  (params (AttachTo :type "SceneComponent Object Reference"))
  ;[1 1 1] Pickup Event
  (`GameplayStatics.SpawnSoundAttached` "/Game/NasaEROSVR/Sounds/plastic_pickup_Cue.plastic_pickup_Cue" (`self.DefaultSceneRoot`) "None" (0.0 0.0 0.0) (struct) "KeepRelativeOffset" false 1.0 1.0 0.0 null null)
  (`SceneComponent.K2_AttachToComponent` (`self.K2_GetRootComponent`) AttachTo "None" "KeepWorld" "KeepWorld" "KeepWorld" false)
  (bind _scannerinterp (`self.ScannerInterp`)
    (:`then`
      (`ActorComponent.K2_DestroyComponent` _scannerinterp)
      (bind _scannerrotate (`self.ScannerRotate`)
        (:`then`
          (`ActorComponent.K2_DestroyComponent` _scannerrotate))
        (:`else`)))
    (:`else`)))

(event `/Game/Blueprints/Character/PickupActorInterface.Drop`
  ;[1 1 1] Drop Event
  (`self.K2_DetachFromActor` "KeepWorld" "KeepWorld" "KeepWorld")
  (`KismetSystemLibrary.Delay` 0.2)
  (bind _returnvalue (`GameplayStatics.GetCurrentLevelName` true))
  (if (`KismetStringLibrary.EqualEqual_StrStr` _returnvalue "Gallery")
    (`self.UpdateTransform`)
    (`/Game/Blueprints/EROS_GameInstance.SaveGame` (`self.GIRef`))))

(event `/Game/VirtualRealityBP/Blueprints/ResizeActorInterface.StartScan`
  ;[1 1 1] Scanning Feature
  (if (and (!= (`self.ScannerCoverObject`) null) (`/Game/Blueprints/EROS_GameInstance.bGalleryObjectsUnlocked` (`self.GIRef`)))
    (bind _returnvalue (`KismetSystemLibrary.K2_SetTimerDelegate` (delegate `HandleScannerTimer`) 0.4))
    (set `self.ScanningTimerHandle` _returnvalue)
    (`GameplayStatics.PlaySound2D` "/Game/NasaEROSVR/Sounds/MinimalUI/370844__cabled-mess__ping-minimal-ui-sounds.370844__cabled-mess__ping-minimal-ui-sounds" 1.0 1.0 0.0 null null)
    (else
      (`/Game/Blueprints/MotionControllerPawn2.ShowNotification` (`self.CharRef`) "<- DataPoints not unlocked ->" (struct :`R` 1.0 :`B` 0.781225 :`A` 1.0)))))

(event `HandleScannerTimer`
  ;[1 1 1] Scanning Feature
  (`self.ScanSuccessful`))

(event `/Game/VirtualRealityBP/Blueprints/ResizeActorInterface.EndScan`
  ;[1 1 1] Scanning Feature
  (`KismetSystemLibrary.K2_ClearAndInvalidateTimerHandle` (`self.ScanningTimerHandle`)))

(event `ScanSuccessful`
  ;[1 1 1] Scanning Feature
  (`ActorComponent.K2_DestroyComponent` (`self.ScannerCoverObject`))
  (`PrimitiveComponent.SetCollisionEnabled` (`self.ScannerCoverObject`) "NoCollision")
  (`GameplayStatics.PlaySound2D` "/Engine/VREditor/Sounds/UI/Camera_Shutter.Camera_Shutter" 1.0 1.0 0.0 null null)
  (`KismetSystemLibrary.K2_ClearAndInvalidateTimerHandle` (`self.RockPulseTimerHandle`))
  (`self.RevealAnimation`)
  (`self.UpdateSaveInformation`))

(event `RevealAnimation`
  ;[1 1 1] Scanner Reveal Animation
  (bind (_direction _newtrack_0) (`Timeline|ScannerRevealTimeline`)
    (:`Update`
      (`self.K2_AddActorWorldOffset` self (`KismetMathLibrary.MakeVector` 0.0 0.0 (`KismetMathLibrary.Lerp` 0.0 2.5 _newtrack_0)) false false)
      (`KismetSystemLibrary.Delay` 1.5)
      (bind _returnvalue (`AddComponent|NODE_AddInterpToMovementComponent-1`))
      (set `self.ScannerInterp` _returnvalue)
      (bind _returnvalue_2 (`AddComponent|NODE_AddRotatingMovementComponent-1`))
      (set `self.ScannerRotate` _returnvalue_2))))

(event `self.ScannerCoverObject.OnComponentBeginOverlap`
  (params (OverlappedComponent :type "PrimitiveComponent Object Reference") (OtherActor :type "Actor Object Reference") (OtherComp :type "PrimitiveComponent Object Reference") (OtherBodyIndex :type Integer) (bFromSweep :type Boolean) (SweepResult :type "HitResult Structure (by ref)"))
  ;[1 1 1] Begin/End Overlap with ScannerPointer
  (bind _outactors (`GameplayStatics.GetAllActorsOfClass` "/Game/Blueprints/MotionControllerPawn2.MotionControllerPawn2_C"))
  (bind _output (`|GetArrayItem` _outactors))
  (if (== (`/Game/Blueprints/MotionControllerPawn2.RController` _output) OtherActor)
    (set `/Game/Blueprints/MotionControllerPawn2.bIsPointingAtScanObject` true _output :!label _label)
    (`/Engine/EditorBlueprintResources/StandardMacros.IncrementInt` (`self.NumControllersPointed`)
      (:`  `
        (set `/Game/Blueprints/MotionControllerPawn2.GalleryObjectPointedAt` self _output)))
    (elif (== (`/Game/Blueprints/MotionControllerPawn2.LController` _output) OtherActor)
      (goto _label))))

(event `self.ScannerCoverObject.OnComponentEndOverlap`
  (params (OverlappedComponent :type "PrimitiveComponent Object Reference") (OtherActor :type "Actor Object Reference") (OtherComp :type "PrimitiveComponent Object Reference") (OtherBodyIndex :type Integer))
  ;[1 1 1] Begin/End Overlap with ScannerPointer
  (bind _outactors (`GameplayStatics.GetAllActorsOfClass` "/Game/Blueprints/MotionControllerPawn2.MotionControllerPawn2_C"))
  (bind _output (`|GetArrayItem` _outactors))
  (if (or (== (`/Game/Blueprints/MotionControllerPawn2.RController` _output) OtherActor) (== (`/Game/Blueprints/MotionControllerPawn2.LController` _output) OtherActor))
    (bind _result (`/Engine/EditorBlueprintResources/StandardMacros.DecrementInt` (`self.NumControllersPointed`))
      (:`  `
        (if (< _result 1)
          (set `/Game/Blueprints/MotionControllerPawn2.bIsPointingAtScanObject` true _output)
          (set `/Game/Blueprints/MotionControllerPawn2.GalleryObjectPointedAt` null _output))))))

(fn `UpdateTransform`
  (returns (CurrentElement :type "/Game/Blueprints/Data/GaleryItemsStruct Structure"))
  (bind (_saveinfo_bisunlocked _saveinfo_currenttransform _saveinfo_currentmesh _saveinfo_currentmaterial _saveinfo_displayedon) (break `/Game/Blueprints/Data/GaleryItemsStruct` (`self.SaveInfo`)))
  ;[1 1 1] UpdateTransform -> called when item released. to save its last known position for loading information.
  (bind _output_get (set `self.SaveInfo` (make `/Game/Blueprints/Data/GaleryItemsStruct` _saveinfo_bisunlocked (`self.GetTransform` self) _saveinfo_currentmesh _saveinfo_currentmaterial _saveinfo_displayedon)))
  (bind _output_get_2 (set `self.CurrentElement` _output_get))
  (return _output_get_2))

(fn `UserConstructionScript`
  (bind (_saveinfo_bisunlocked _saveinfo_currenttransform _saveinfo_currentmesh _saveinfo_currentmaterial) (break `/Game/Blueprints/Data/GaleryItemsStruct` (`self.SaveInfo`)))
  (bind _staticmesh (`self.StaticMesh`))
  (`StaticMeshComponent.SetStaticMesh` _staticmesh _saveinfo_currentmesh)
  (`PrimitiveComponent.SetMaterial` _staticmesh 0 _saveinfo_currentmaterial))

(fn `WhatsMyName`
  (returns (Output_Get :type Text))
  (bind _output_get (set `self.MyName` (`KismetTextLibrary.Conv_StringToText` (`KismetStringLibrary.Concat_StrStr` (`KismetSystemLibrary.GetDisplayName` self) " Gallery Object Unlocked"))))
  (return _output_get))