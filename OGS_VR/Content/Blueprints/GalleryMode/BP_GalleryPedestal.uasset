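; VR gallery pedestal that displays a dropped BP_PickupCube and lets the player rotate it.
; Box overlap makes both motion controllers release, then a timeline pulls the item to the box with particles and sound; leaving clears it.
; Controller grab spheres overlapping LControl or RControl run looping timers that yaw the item, one direction at a time.
; Gallery save-info updates are ineffective: one follows clearing the item reference, another is unwired.
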(event `self.RControl.OnComponentBeginOverlap`
  (params (OverlappedComponent :type "PrimitiveComponent Object Reference") (OtherActor :type "Actor Object Reference") (OtherComp :type "PrimitiveComponent Object Reference") (OtherBodyIndex :type Integer) (bFromSweep :type Boolean) (SweepResult :type "HitResult Structure (by ref)"))
  ;[1 1 1] Overlap events for rotation control spheres
  (bind _asbp_motion_controller_2 (cast `/Game/Blueprints/Character/BP_MotionController2` OtherActor))
  (if (== OtherComp (`/Game/Blueprints/Character/BP_MotionController2.GrabSphere` _asbp_motion_controller_2))
    (`GameplayStatics.PlaySound2D` "/Game/NasaEROSVR/Sounds/MinimalUI/370844__cabled-mess__ping-minimal-ui-sounds.370844__cabled-mess__ping-minimal-ui-sounds" 1.0 1.0 0.0 null null)
    (bind _returnvalue (`KismetSystemLibrary.K2_SetTimerDelegate` (delegate `HandleLRotationTimer`) 0.01 true))
    (set `self.LRotationTimer` _returnvalue)))

(event `self.LRotateSphereCollision.OnComponentBeginOverlap`
  (params (OverlappedComponent :type "PrimitiveComponent Object Reference") (OtherActor :type "Actor Object Reference") (OtherComp :type "PrimitiveComponent Object Reference") (OtherBodyIndex :type Integer) (bFromSweep :type Boolean) (SweepResult :type "HitResult Structure (by ref)"))
  ;[1 1 1] Overlap events for rotation control spheres
)

(event `LRotationEvent`
  (bind _itemtocontrol (`self.ItemToControl`))
  ;[1 1 1] Rotate the gallery item
  (if (!= _itemtocontrol null)
    (if (not (`self.bIsRotatingRight`))
      (set `self.bIsRotatingLeft` true)
      ;[1 0.2654 0] pivot points should maybe be in the center of the mesh
      (`SceneComponent.K2_AddLocalRotation` (`Actor.RootComponent` _itemtocontrol) (struct :`Yaw` -1.0) false false))))

(event `self.RControl.OnComponentEndOverlap`
  (params (OverlappedComponent :type "PrimitiveComponent Object Reference") (OtherActor :type "Actor Object Reference") (OtherComp :type "PrimitiveComponent Object Reference") (OtherBodyIndex :type Integer))
  ;[1 1 1] Overlap events for rotation control spheres
  (bind _asbp_motion_controller_2 (cast `/Game/Blueprints/Character/BP_MotionController2` OtherActor))
  (if (== OtherComp (`/Game/Blueprints/Character/BP_MotionController2.GrabSphere` _asbp_motion_controller_2))
    (`KismetSystemLibrary.K2_ClearAndInvalidateTimerHandle` (`self.LRotationTimer`))
    (set `self.bIsRotatingLeft` false)))

(event `self.LRotateSphereCollision.OnComponentEndOverlap`
  (params (OverlappedComponent :type "PrimitiveComponent Object Reference") (OtherActor :type "Actor Object Reference") (OtherComp :type "PrimitiveComponent Object Reference") (OtherBodyIndex :type Integer))
  ;[1 1 1] Overlap events for rotation control spheres
)

(event `HandleLRotationTimer`
  ;[1 1 1] Overlap events for rotation control spheres
  (`self.LRotationEvent`))

(event `RRotationEvent`
  ;[1 1 1] Rotate the gallery item
  (if (!= (`self.ItemToControl`) null)
    (if (not (`self.bIsRotatingLeft`))
      (set `self.bIsRotatingRight` true)
      ;[1 0.2654 0] pivot points should maybe be in the center of the mesh
      (`SceneComponent.K2_AddLocalRotation` (`Actor.RootComponent` (`self.ItemToControl`)) (struct :`Yaw` 1.0) false false))))

(event `self.LControl.OnComponentBeginOverlap`
  (params (OverlappedComponent :type "PrimitiveComponent Object Reference") (OtherActor :type "Actor Object Reference") (OtherComp :type "PrimitiveComponent Object Reference") (OtherBodyIndex :type Integer) (bFromSweep :type Boolean) (SweepResult :type "HitResult Structure (by ref)"))
  ;[1 1 1] Overlap events for rotation control spheres
  (bind _asbp_motion_controller_2 (cast `/Game/Blueprints/Character/BP_MotionController2` OtherActor))
  (if (== OtherComp (`/Game/Blueprints/Character/BP_MotionController2.GrabSphere` _asbp_motion_controller_2))
    (`GameplayStatics.PlaySound2D` "/Game/NasaEROSVR/Sounds/MinimalUI/370844__cabled-mess__ping-minimal-ui-sounds.370844__cabled-mess__ping-minimal-ui-sounds" 1.0 1.0 0.0 null null)
    (bind _returnvalue (`KismetSystemLibrary.K2_SetTimerDelegate` (delegate `HandleRRotationTimer`) 0.01 true))
    (set `self.RRotationTimer` _returnvalue)))

(event `self.RRotateSphereCollision.OnComponentBeginOverlap`
  (params (OverlappedComponent :type "PrimitiveComponent Object Reference") (OtherActor :type "Actor Object Reference") (OtherComp :type "PrimitiveComponent Object Reference") (OtherBodyIndex :type Integer) (bFromSweep :type Boolean) (SweepResult :type "HitResult Structure (by ref)"))
  ;[1 1 1] Overlap events for rotation control spheres
)

(event `self.LControl.OnComponentEndOverlap`
  (params (OverlappedComponent :type "PrimitiveComponent Object Reference") (OtherActor :type "Actor Object Reference") (OtherComp :type "PrimitiveComponent Object Reference") (OtherBodyIndex :type Integer))
  ;[1 1 1] Overlap events for rotation control spheres
  (bind _asbp_motion_controller_2 (cast `/Game/Blueprints/Character/BP_MotionController2` OtherActor))
  (if (== OtherComp (`/Game/Blueprints/Character/BP_MotionController2.GrabSphere` _asbp_motion_controller_2))
    (`KismetSystemLibrary.K2_ClearAndInvalidateTimerHandle` (`self.RRotationTimer`))
    (set `self.bIsRotatingRight` false)))

(event `self.RRotateSphereCollision.OnComponentEndOverlap`
  (params (OverlappedComponent :type "PrimitiveComponent Object Reference") (OtherActor :type "Actor Object Reference") (OtherComp :type "PrimitiveComponent Object Reference") (OtherBodyIndex :type Integer))
  ;[1 1 1] Overlap events for rotation control spheres
)

(event `HandleRRotationTimer`
  ;[1 1 1] Overlap events for rotation control spheres
  (`self.RRotationEvent`))

(event `self.Box.OnComponentBeginOverlap`
  (params (OverlappedComponent :type "PrimitiveComponent Object Reference") (OtherActor :type "Actor Object Reference") (OtherComp :type "PrimitiveComponent Object Reference") (OtherBodyIndex :type Integer) (bFromSweep :type Boolean) (SweepResult :type "HitResult Structure (by ref)"))
  (bind _rootcomponent (`Actor.RootComponent` (`self.ItemToControl`)))
  ;[1 1 1] move items of pickupcube or child classes to pedestal if not filled, play sound and activate particle effect.
  (if (not (`self.bPedestalFilled`))
    (bind _asbp_pickup_cube (cast `/Game/Blueprints/BP_PickupCube` OtherActor))
    (set `self.ItemToControl` _asbp_pickup_cube)
    (bind _asmotion_controller_pawn_2 (cast `/Game/Blueprints/MotionControllerPawn2` (`GameplayStatics.GetPlayerCharacter` 0))
      (:`then`
        (`/Game/Blueprints/Character/BP_MotionController2.ReleaseActor` (`/Game/Blueprints/MotionControllerPawn2.LController` _asmotion_controller_pawn_2))
        (`/Game/Blueprints/Character/BP_MotionController2.ReleaseActor` (`/Game/Blueprints/MotionControllerPawn2.RController` _asmotion_controller_pawn_2))
        (bind (_direction _newtrack_0) (`Timeline|Timeline_0` :!via `PlayFromStart`)
          (:`Update`
            (`SceneComponent.K2_SetWorldLocation` _rootcomponent (`KismetMathLibrary.VLerp` (`SceneComponent.K2_GetComponentLocation` _rootcomponent) (`SceneComponent.K2_GetComponentLocation` (`self.Box`)) _newtrack_0) false false)
            (`ActorComponent.Activate` (`self.ParticleSystem`) false))
          (:`Finished`
            (`GameplayStatics.PlaySound2D` "/Engine/VREditor/Sounds/UI/Camera_Shutter.Camera_Shutter" 1.0 1.0 0.0 null null)
            (set `self.bPedestalFilled` true))))
      (:`CastFailed`
        (`GameplayStatics.PlaySound2D` "/Game/NasaEROSVR/Sounds/metal_hit1.metal_hit1" 1.0 1.0 0.0 null null)))))

(event `self.Box.OnComponentEndOverlap`
  (params (OverlappedComponent :type "PrimitiveComponent Object Reference") (OtherActor :type "Actor Object Reference") (OtherComp :type "PrimitiveComponent Object Reference") (OtherBodyIndex :type Integer))
  ;[1 1 1] remove currently displayed item, play sound, and deactivate particle effect.
  (if (== OtherActor (`self.ItemToControl`))
    (set `self.bPedestalFilled` false)
    (set `self.ItemToControl` null)
    (`GameplayStatics.PlaySound2D` "/Engine/VREditor/Sounds/VR_negative.VR_negative" 0.4 1.0 0.0 null null)
    (`ActorComponent.Deactivate` (`self.ParticleSystem`))
    (bind _asbp_gallery_item_2 (cast `/Game/Blueprints/GalleryMode/BP_GalleryItem2` (`self.ItemToControl`)))
    (bind (_saveinfo_bisunlocked _saveinfo_currenttransform _saveinfo_currentmesh _saveinfo_currentmaterial) (break `/Game/Blueprints/Data/GaleryItemsStruct` (`/Game/Blueprints/GalleryMode/BP_GalleryItem2.SaveInfo` _asbp_gallery_item_2)))
    (set `/Game/Blueprints/GalleryMode/BP_GalleryItem2.SaveInfo` (make `/Game/Blueprints/Data/GaleryItemsStruct` _saveinfo_bisunlocked _saveinfo_currenttransform _saveinfo_currentmesh _saveinfo_currentmaterial) _asbp_gallery_item_2)))

(fn `UserConstructionScript`)