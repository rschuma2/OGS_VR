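; BP_WorldWidget is an actor that displays a configurable UMG widget in the world through its widget component.
; On BeginPlay it scales the component, waits a set spawn delay, then creates the chosen widget class and assigns it to the component.
; After the delay it also clears menu mode and re-enables turning on the player's MotionControllerPawn2; a failed cast stops the widget being created.
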(event `self.ReceiveBeginPlay`
  (`SceneComponent.SetWorldScale3D` (`self.Widget`) (`self.WidgetScale`))
  (`KismetSystemLibrary.Delay` (`self.WidgetSpawnDelay`))
  ;[1 0.51 0] Turn off 'menu mode' to allow movement add to controllerpawn
  (bind _asmotion_controller_pawn_2 (cast `/Game/Blueprints/MotionControllerPawn2` (`GameplayStatics.GetPlayerCharacter` 0)))
  (set `/Game/Blueprints/MotionControllerPawn2.bIsInMenu` false _asmotion_controller_pawn_2)
  (set `/Game/Blueprints/MotionControllerPawn2.canTurn` true _asmotion_controller_pawn_2)
  (bind _returnvalue (`|CreateWidget` (`self.WidgetToLoad`)))
  (bind _output_get (set `self.WorldWidget` _returnvalue))
  (`WidgetComponent.SetWidget` (`self.Widget`) _output_get))

(fn `UserConstructionScript`
  (`parent.UserConstructionScript`))