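; BP_ScannerButton is a wrist UI button that toggles the player's scanner on and off.
; Each ButtonAction call alternates through a FlipFlop, playing a distinct UI sound and setting ScanIsUnlocked and ReadyToScan on the player's MotionControllerPawn2.
; The button's Cube swaps between an emissive material when on and the basic shape material when off.
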(event `self.ButtonAction`
  (`/Engine/EditorBlueprintResources/StandardMacros.FlipFlop`
    (:`A`
      (`GameplayStatics.PlaySound2D` "/Game/NasaEROSVR/Sounds/MinimalUI/370844__cabled-mess__ping-minimal-ui-sounds.370844__cabled-mess__ping-minimal-ui-sounds" 1.0 1.0 0.0 null null)
      (bind _asmotion_controller_pawn_2 (cast `/Game/Blueprints/MotionControllerPawn2` (`GameplayStatics.GetPlayerCharacter` 0)))
      (set `/Game/Blueprints/MotionControllerPawn2.bScanIsUnlocked` true _asmotion_controller_pawn_2)
      (set `/Game/Blueprints/MotionControllerPawn2.ReadyToScan` true _asmotion_controller_pawn_2)
      (`PrimitiveComponent.SetMaterial` (`self.Cube`) 0 "/Engine/ArtTools/RenderToTexture/Materials/Debug/M_Emissive_Color_0-0-127.M_Emissive_Color_0-0-127"))
    (:`B`
      (`GameplayStatics.PlaySound2D` "/Game/NasaEROSVR/Sounds/MinimalUI/370846__cabled-mess__funny-click-minimal-ui-sounds.370846__cabled-mess__funny-click-minimal-ui-sounds" 1.0 1.0 0.0 null null)
      (bind _asmotion_controller_pawn_2_2 (cast `/Game/Blueprints/MotionControllerPawn2` (`GameplayStatics.GetPlayerCharacter` 0)))
      (set `/Game/Blueprints/MotionControllerPawn2.bScanIsUnlocked` false _asmotion_controller_pawn_2_2)
      (set `/Game/Blueprints/MotionControllerPawn2.ReadyToScan` false _asmotion_controller_pawn_2_2)
      (`PrimitiveComponent.SetMaterial` (`self.Cube`) 0 "/Engine/BasicShapes/BasicShapeMaterial.BasicShapeMaterial"))))

(fn `UserConstructionScript`
  (`parent.UserConstructionScript`))