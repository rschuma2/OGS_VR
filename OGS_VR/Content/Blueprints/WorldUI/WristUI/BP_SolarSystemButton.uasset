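; Wrist UI button that switches between the SolarSystemMap level and the game's current level.
; At begin play it checks the level name and sets its label, showing a back-to-Eros text when already on the map.
; On press it plays a ping and, after a brief delay, opens the map or the level name stored in GIRef.
; If GIRef.SolarSystemUnlocked is false, it plays a failure sound instead.
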(event `self.ChildBeginPlay`
  ;[1 1 1] BeginPlay. Set text based on location
  (bind _returnvalue (`GameplayStatics.GetCurrentLevelName` true))
  (if (`KismetStringLibrary.EqualEqual_StrStr` _returnvalue "SolarSystemMap")
    (set `self.bIsOnSolarSystemMap` true)
    (`TextRenderComponent.K2_SetText` (`self.TextRender`) (`self.BackToEros`))
    (else
      (`TextRenderComponent.K2_SetText` (`self.TextRender`) (`self.ButtonText`)))))

(event `self.ButtonAction`
  ;[1 1 1] Button Action
  (`GameplayStatics.PlaySound2D` "/Game/NasaEROSVR/Sounds/MinimalUI/370844__cabled-mess__ping-minimal-ui-sounds.370844__cabled-mess__ping-minimal-ui-sounds" 1.0 1.0 0.0 null null)
  (`KismetSystemLibrary.Delay` 0.2)
  (if (`/Game/Blueprints/EROS_GameInstance.bSolarSystemUnlocked` (`self.GIRef`))
    (if (`self.bIsOnSolarSystemMap`)
      (`GameplayStatics.OpenLevel` (`/Game/Blueprints/EROS_GameInstance.CurrentLevelName` (`self.GIRef`)))
      (else
        (`GameplayStatics.OpenLevel` "SolarSystemMap")))
    (else
      (`GameplayStatics.PlaySound2D` "/Engine/EditorSounds/Notifications/CompileFailed.CompileFailed" 1.0 1.0 0.0 null null))))

(fn `UserConstructionScript`
  (`parent.UserConstructionScript`))